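; Player ninja character with constant forward movement, strafing, crouch, double jump, dash, punches and thrown ninja stars.
; Tick runs side and forward line traces while falling to drive wall runs and wall clings, altering gravity and plane constraints.
; Jump input launches off walls or double-jumps, and OffWall restores gravity and dash.
; Punch montage notifies toggle hand collision components that apply damage on overlap.
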(event OnComponentBeginOverlap(AttackDMGRight)
  (params (OverlappedComponent :type Primitive%20Component%20Object%20Reference) (OtherActor :type Actor%20Object%20Reference) (OtherComp :type Primitive%20Component%20Object%20Reference) (OtherBodyIndex :type Integer) (bFromSweep :type Boolean) (SweepResult :type Hit%20Result%20Structure%20%28by%20ref%29))
  ;[0 0 0] Attack
  ;;[1 0.2044 0] Applying DMG for Jab Cros
  (Game|Damage|ApplyDamage OtherActor 2e+01 0 self))

(event OnComponentBeginOverlap(AttackDMGLeft)
  (params (OverlappedComponent :type Primitive%20Component%20Object%20Reference) (OtherActor :type Actor%20Object%20Reference) (OtherComp :type Primitive%20Component%20Object%20Reference) (OtherBodyIndex :type Integer) (bFromSweep :type Boolean) (SweepResult :type Hit%20Result%20Structure%20%28by%20ref%29))
  ;[0 0 0] Attack
  ;;[1 0.2044 0] Applying DMG for Jab Cros
  (Game|Damage|ApplyDamage OtherActor 1e+01 0 self))

(event Custom|offWall
  (bind _charactermovement (Variables|Character|GetCharacterMovement))
  ;[0 0 0] Custom Events
  ;;[1 0 0] offWall
  (Variables|/Script/Engine.CharacterMovementComponent|SetGravityScale _charactermovement 1.0)
  (Class|MovementComponent|SetPlaneConstraintNormal _charactermovement (Math|Vector|MakeVector 0.0 0.0 0.0))
  (Variables|Dashing|SetcanDash? true))

(event Custom|resetDash
  (bind _returnvalue (Transformation|GetActorForwardVector))
  ;[0 0 0] Character Movement
  ;;[0 0.9841 1] Dash
  (Utilities|FlowControl|DoOnce false) ; enters at Reset
)

(event Input|EnhancedActionEvents|EnhancedInputActionIA-Move
  (params (ActionValue :type Vector%202D%20Structure) (ElapsedSeconds :type Float%20%28double-precision%29) (TriggeredSeconds :type Float%20%28double-precision%29) (InputAction :type Input%20Action%20Object%20Reference :default "/Game/Input/InputAction/IA-Move.IA-Move"))
  ;[0 0 0] Character Movement
  ;;[0 0.9841 1] Move
  (Pawn|Input|AddMovementInput (Math|Vector|GetRightVector (Math|Rotator|MakeRotator 0.0 0.0 (.yaw (Pawn|GetControlRotation :!class /Script/Engine.Pawn)))) (.x ActionValue) false))

(event Input|EnhancedActionEvents|EnhancedInputActionIA-Jump
  (params (ActionValue :type Boolean) (ElapsedSeconds :type Float%20%28double-precision%29) (TriggeredSeconds :type Float%20%28double-precision%29) (InputAction :type Input%20Action%20Object%20Reference :default "/Game/Input/InputAction/IA-Jump.IA-Jump"))
  (bind _returnvalue (Transformation|GetActorRotation))
  (bind _returnvalue_2 (Transformation|GetActorForwardVector))
  (bind _returnvalue_3 (Transformation|GetActorRightVector))
  (bind _onrightside (Variables|WallRunning|GetonRightSide))
  (bind _charactermovement (Variables|Character|GetCharacterMovement))
  (bind _returnvalue_4 (* _returnvalue_3 6e+02))
  (bind _returnvalue_5 (* _returnvalue_3 -6e+02))
  (bind _returnvalue_6 (* _returnvalue_2 -1.8e+03))
  (bind _jumpzvelocity (Variables|/Script/Engine.CharacterMovementComponent|GetJumpZVelocity _charactermovement))
  (bind _returnvalue_7 (select _onrightside _returnvalue_5 _returnvalue_4))
  ;[0 0 0] Character Movement
  ;;[0 0.9841 1] Jumping
  (:Triggered
    (Utilities|FlowControl|Sequence
      (:then_0
        (if (or (Variables|WallRunning|GetrightSide) (Variables|WallRunning|GetleftSide))
          (Variables|WallRunning|SetisJumpingOffWall true)
          (CallFunction|OffWall)
          (Utilities|FlowControl|DoOnce false :!label _label
            (:Completed
              (Character|LaunchCharacter (Math|Vector|MakeVector (.x _returnvalue_7) (.y _returnvalue_7) _jumpzvelocity) false true)
              (Utilities|FlowControl|Delay 0.5)
              (Variables|WallRunning|SetisJumpingOffWall false)
              (goto _label Reset)))
          (else
            (Character|Jump)
            (if (and (AI|Components|NavMovement|IsFalling (Variables|Character|GetCharacterMovement)) (Variables|Default|GetcanDoubleJump?))
              (Variables|Default|SetcanDoubleJump? false)
              (Character|LaunchCharacter (Math|Vector|MakeVector 0.0 0.0 _jumpzvelocity) false true)))))
      (:then_1
        (if (Variables|WallJump|GetstuckToWall?)
          (Variables|WallRunning|SetisJumpingOffWall true)
          (CallFunction|OffWall)
          (Utilities|FlowControl|DoOnce false :!label _label_2
            (:Completed
              (Character|LaunchCharacter (Math|Vector|MakeVector (.x _returnvalue_6) (.y _returnvalue_6) (Variables|/Script/Engine.CharacterMovementComponent|GetJumpZVelocity (Variables|Character|GetCharacterMovement))) false false)
              (Transformation|SetActorRotation (Math|Rotator|MakeRotator (.roll _returnvalue) (.pitch _returnvalue) (+ (.yaw _returnvalue) 1.8e+02)))
              (Utilities|FlowControl|Delay 0.5)
              (Variables|WallRunning|SetisJumpingOffWall false)
              (goto _label_2 Reset)))))))
  (:Completed
    (Character|StopJumping)))

(event Input|EnhancedActionEvents|EnhancedInputActionIA-Look
  (params (ActionValue :type Vector%202D%20Structure) (ElapsedSeconds :type Float%20%28double-precision%29) (TriggeredSeconds :type Float%20%28double-precision%29) (InputAction :type Input%20Action%20Object%20Reference :default "/Game/Input/InputAction/IA-Look.IA-Look"))
  ;[0 0 0] Character Movement
  ;;[0 0.9841 1] Look
  (Pawn|Input|AddControllerYawInput (.x ActionValue))
  (Pawn|Input|AddControllerPitchInput (* (.y ActionValue) -1.0)))

(event Input|EnhancedActionEvents|EnhancedInputActionIA-Punch
  (params (ActionValue :type Boolean) (ElapsedSeconds :type Float%20%28double-precision%29) (TriggeredSeconds :type Float%20%28double-precision%29) (InputAction :type Input%20Action%20Object%20Reference :default "/Game/Input/InputAction/IA-Punch.IA-Punch"))
  ;[0 0 0] Attack
  ;;[1 0.2044 0] Attack (Jab Cross)
  (:Started
    (if (not (and (AI|Components|NavMovement|IsCrouching (Variables|Character|GetCharacterMovement)) (Variables|Default|Getaiming?)))
      (switch Utilities|FlowControl|Switch|SwitchonEMovementMode (Variables|/Script/Engine.CharacterMovementComponent|GetMovementMode (Variables|Character|GetCharacterMovement))
        (:MOVE_Walking
          (Pawn|Components|CharacterMovement|SetMovementMode (Variables|Character|GetCharacterMovement) "MOVE_None" 0)
          (bind _notifyname (Animation|Montage|PlayMontage (Variables|Character|GetMesh) "/Game/Mixamo/Animations/Jab_Cross_Montage.Jab_Cross_Montage")
            (:OnNotifyBegin
              (switch name _notifyname
                (:St_LeftH
                  (Collision|SetCollisionProfileName (Variables|Default|GetAttack%20DMG%20Left) "None" true :!class /Script/Engine.PrimitiveComponent))
                (:Stp_LeftH
                  (Collision|SetCollisionProfileName (Variables|Default|GetAttack%20DMG%20Left) "NoCollision" true :!class /Script/Engine.PrimitiveComponent))
                (:St_RightH
                  (Collision|SetCollisionProfileName (Variables|Default|GetAttack%20DMG%20Right) "OverlapAllDynamic" true :!class /Script/Engine.PrimitiveComponent))
                (:Stp_RightH
                  (Collision|SetCollisionProfileName (Variables|Default|GetAttack%20DMG%20Right) "NoCollision" true :!class /Script/Engine.PrimitiveComponent))
                (:Start%20Moving
                  (Pawn|Components|CharacterMovement|SetMovementMode (Variables|Character|GetCharacterMovement) "MOVE_Walking" 0))))))))))

(event Input|EnhancedActionEvents|EnhancedInputActionIA-Crouch
  (params (ActionValue :type Boolean) (ElapsedSeconds :type Float%20%28double-precision%29) (TriggeredSeconds :type Float%20%28double-precision%29) (InputAction :type Input%20Action%20Object%20Reference :default "/Game/Input/InputAction/IA-Crouch.IA-Crouch"))
  ;[0 0 0] Character Movement
  ;;[0 0.9841 1] Crouch
  (:Started
    (Character|Crouch))
  (:Completed
    (Character|UnCrouch)))

(event Input|EnhancedActionEvents|EnhancedInputActionIA-Run
  (params (ActionValue :type Boolean) (ElapsedSeconds :type Float%20%28double-precision%29) (TriggeredSeconds :type Float%20%28double-precision%29) (InputAction :type Input%20Action%20Object%20Reference :default "/Game/Input/InputAction/IA-Run.IA-Run"))
  (bind _returnvalue (Transformation|GetActorForwardVector))
  ;[0 0 0] Character Movement
  ;;[0 0.9841 1] Dash
  (Utilities|FlowControl|DoOnce false :!label _label
    (:Completed
      (if (Variables|Dashing|GetcanDash?)
        (Variables|Dashing|SetisDashing true)
        (Variables|/Script/Engine.CharacterMovementComponent|SetGroundFriction (Variables|Character|GetCharacterMovement) 3.0)
        (Character|LaunchCharacter (Math|Vector|MakeVector (* (.x _returnvalue) 7e+03) (* (.y _returnvalue) 7e+03) 0.0) false true)
        (Variables|Dashing|SetisDashing false)
        (CallFunction|OffWall)
        (Variables|/Script/Engine.CharacterMovementComponent|SetGroundFriction (Variables|Character|GetCharacterMovement) 8.0)
        (Utilities|FlowControl|Delay 1.0)
        (goto _label Reset)))))

(event Input|EnhancedActionEvents|EnhancedInputActionIA-Dash
  (params (ActionValue :type Boolean) (ElapsedSeconds :type Float%20%28double-precision%29) (TriggeredSeconds :type Float%20%28double-precision%29) (InputAction :type Input%20Action%20Object%20Reference :default "/Game/Input/InputAction/IA-Dash.IA-Dash"))
  ;[0.02832 0 1] Sprint (Not in use)
)

(event Input|EnhancedActionEvents|EnhancedInputActionIA-Aim
  (params (ActionValue :type Boolean) (ElapsedSeconds :type Float%20%28double-precision%29) (TriggeredSeconds :type Float%20%28double-precision%29) (InputAction :type Input%20Action%20Object%20Reference :default "/Game/Input/InputAction/IA-Aim.IA-Aim"))
  (bind _scene (Variables|Default|GetScene))
  ;[0 0 0] Attack
  ;;[1 0.2044 0] Aim
  (Game|SpawnActorfromClass "/Game/Actors/Projectiles/BP_ninjaStar.BP_ninjaStar_C" (Math|Transform|MakeTransform (Transformation|GetWorldLocation _scene) (Transformation|GetWorldRotation _scene) "0.200000,0.200000,0.200000") "Undefined" "MultiplyWithRoot" 0 1.6e+03 0.0 0))

(event EventBeginPlay
  ;[0 0 0] Event Calls
  ;;[0 1 0.02998] Get character to add mapping context
  (Class|MovementComponent|SetPlaneConstraintEnabled (Variables|Character|GetCharacterMovement) true)
  (bind _asplayer_controller (Utilities|Casting|CastToPlayerController (Pawn|GetController)))
  (Utilities|IsValid _asplayer_controller
    (:Is%20Valid
      (Input|AddMappingContext (PlayerController|LocalPlayerSubsystems|GetEnhancedInputLocalPlayerSubsystem _asplayer_controller) "/Game/Input/IMC_Ninja.IMC_Ninja" 0 "(bIgnoreAllPressedKeysUntilRelease=True,bForceImmediately=False,bNotifyUserSettings=False)"))))

(event EventTick
  (params (DeltaSeconds :type Float%20%28single-precision%29))
  ;[0 0 0] Event Calls
  ;;[0 1 0.02998] Event Tick
  (CallFunction|WallRun)
  (CallFunction|WallJump))

(event EventOnLanded
  (params (Hit :type Hit%20Result%20Structure%20%28by%20ref%29))
  ;[0 0 0] Event Calls
  ;;[0 1 0.02998] Event On Landed
  (Variables|Default|SetcanDoubleJump? true))

(event EventAsyncPhysicsTick
  (params (DeltaSeconds :type Float%20%28single-precision%29) (SimSeconds :type Float%20%28single-precision%29))
  ;[0 0 0] Character Movement
  ;;[0 0.9841 1] Move
  (Pawn|Input|AddMovementInput (Math|Vector|GetForwardVector (Math|Rotator|MakeRotator 0.0 0.0 (.yaw (Pawn|GetControlRotation :!class /Script/Engine.Pawn)))) 1.0 false))

(fn ConstructionScript)

(fn BPNinjaAutoGenFunc
  (params (SelfActor :type Actor%20Object%20Reference) (OtherActor :type Actor%20Object%20Reference) (NormalImpulse :type Vector) (Hit :type Hit%20Result%20Structure%20%28by%20ref%29))
  (return))

(fn WallRun
  (bind _returnvalue (Transformation|GetActorLocation))
  (bind _returnvalue_2 (Transformation|GetActorLocation))
  (bind _returnvalue_3 (Transformation|GetActorForwardVector))
  (bind _returnvalue_4 (Transformation|GetActorForwardVector))
  (bind _charactermovement (Variables|Character|GetCharacterMovement))
  (bind _charactermovement_2 (Variables|Character|GetCharacterMovement))
  (bind _charactermovement_3 (Variables|Character|GetCharacterMovement))
  (bind _returnvalue_5 (* _returnvalue_4 5e+02))
  (bind _returnvalue_6 (* _returnvalue_3 5e+02))
  (if (Math|Boolean|ANDBoolean (AI|Components|NavMovement|IsFalling _charactermovement_3) (<= (.z (Variables|/Script/Engine.MovementComponent|GetVelocity _charactermovement_3)) 0.0) (and (< (.x (Variables|/Script/Engine.MovementComponent|GetVelocity _charactermovement_3)) 501.0) (< (.y (Variables|/Script/Engine.MovementComponent|GetVelocity _charactermovement_3)) 501.0)))
    (Utilities|FlowControl|Sequence
      (:then_0
        ;[0 0 0] Right Wall Run
        (if (not (Variables|WallRunning|GetleftSide))
          (bind (_outhit _returnvalue_7) (Collision|LineTraceByChannel _returnvalue_2 (+ _returnvalue_2 (* (Transformation|GetActorRightVector) 5e+01)) "TraceTypeQuery3" false 0 "ForOneFrame"))
          (if _returnvalue_7
            (Animation|StopAnimMontage "/Game/Mixamo/Animations/RunningSlide_UE_Montage.RunningSlide_UE_Montage")
            (Variables|Dashing|SetcanDash? false)
            (Variables|WallRunning|SetrightSide true)
            (Variables|WallRunning|SetonRightSide true)
            (if (not (Variables|WallRunning|GetisJumpingOffWall))
              (Transformation|SetActorRotation (Math|Rotator|MakeRotator 0.0 0.0 (+ (.yaw (Math|Conversions|RotationFromXVector (.Normal (Collision|BreakHitResult _outhit)))) 9e+01)))
              (Variables|/Script/Engine.MovementComponent|SetVelocity _charactermovement_2 (Math|Vector|MakeVector (.x _returnvalue_5) (.y _returnvalue_5) 0.0))
              (Variables|/Script/Engine.CharacterMovementComponent|SetGravityScale _charactermovement_2 0.0)
              (Class|MovementComponent|SetPlaneConstraintNormal _charactermovement_2 "0.000000,0.000000,1.000000")
              (Variables|Dashing|SetcanDash? false)
              (Variables|Default|SetcanDoubleJump? true))
            (else
              (Variables|WallRunning|SetrightSide false)
              (CallFunction|OffWall)))))
      (:then_1
        ;[0 0 0] Left Wall Run
        (if (not (Variables|WallRunning|GetrightSide))
          (bind (_outhit_2 _returnvalue_8) (Collision|LineTraceByChannel _returnvalue (+ _returnvalue (* (Transformation|GetActorRightVector) -5e+01)) "TraceTypeQuery3" false 0 "ForOneFrame"))
          (if _returnvalue_8
            (Animation|StopAnimMontage "/Game/Mixamo/Animations/RunningSlide_UE_Montage.RunningSlide_UE_Montage")
            (Variables|Dashing|SetcanDash? false)
            (Variables|WallRunning|SetleftSide true)
            (Variables|WallRunning|SetonRightSide false)
            (if (not (Variables|WallRunning|GetisJumpingOffWall))
              (Transformation|SetActorRotation (Math|Rotator|MakeRotator 0.0 0.0 (+ -9e+01 (.yaw (Math|Conversions|RotationFromXVector (.Normal (Collision|BreakHitResult _outhit_2)))))))
              (Variables|/Script/Engine.MovementComponent|SetVelocity _charactermovement (Math|Vector|MakeVector (.x _returnvalue_6) (.y _returnvalue_6) 0.0))
              (Variables|/Script/Engine.CharacterMovementComponent|SetGravityScale _charactermovement 0.0)
              (Class|MovementComponent|SetPlaneConstraintNormal _charactermovement "0.000000,0.000000,1.000000")
              (Variables|Dashing|SetcanDash? false)
              (Variables|Default|SetcanDoubleJump? true))
            (else
              (Variables|WallRunning|SetleftSide false)
              (CallFunction|OffWall))))))))

(fn WallJump
  (bind _returnvalue (Transformation|GetActorLocation))
  (bind _charactermovement (Variables|Character|GetCharacterMovement))
  (bind _charactermovement_2 (Variables|Character|GetCharacterMovement))
  (if (Math|Boolean|ANDBoolean (AI|Components|NavMovement|IsFalling _charactermovement) (<= (.z (Variables|/Script/Engine.MovementComponent|GetVelocity _charactermovement)) 0.0) (and (< (.x (Variables|/Script/Engine.MovementComponent|GetVelocity _charactermovement)) 501.0) (< (.y (Variables|/Script/Engine.MovementComponent|GetVelocity _charactermovement)) 501.0)))
    (bind (_outhit _returnvalue_2) (Collision|LineTraceByChannel _returnvalue (+ _returnvalue (* (Transformation|GetActorForwardVector) 5e+01)) "TraceTypeQuery4" false 0 "ForOneFrame"))
    (if _returnvalue_2
      (Variables|WallJump|SetstuckToWall? true)
      (Transformation|SetActorRotation (Math|Rotator|MakeRotator 0.0 0.0 (+ (.yaw (Math|Conversions|RotationFromXVector (.Normal (Collision|BreakHitResult _outhit)))) 1.8e+02)))
      (Variables|/Script/Engine.MovementComponent|SetVelocity _charactermovement_2 (Math|Vector|MakeVector 0.0 0.0 0.0))
      (Variables|/Script/Engine.CharacterMovementComponent|SetGravityScale _charactermovement_2 4.0)
      (Class|MovementComponent|SetPlaneConstraintNormal _charactermovement_2 "1.000000,1.000000,0.000000")
      (else
        (CallFunction|OffWall)
        (Variables|WallJump|SetstuckToWall? false)))))

(fn IA-Jump
  (bind _returnvalue (Transformation|GetActorRotation))
  (bind _returnvalue_2 (Transformation|GetActorForwardVector))
  (bind _returnvalue_3 (Transformation|GetActorRightVector))
  (bind _onrightside (Variables|WallRunning|GetonRightSide))
  (bind _charactermovement (Variables|Character|GetCharacterMovement))
  (bind _returnvalue_4 (* _returnvalue_3 6e+02))
  (bind _returnvalue_5 (* _returnvalue_3 -6e+02))
  (bind _returnvalue_6 (* _returnvalue_2 -1.8e+03))
  (bind _jumpzvelocity (Variables|/Script/Engine.CharacterMovementComponent|GetJumpZVelocity _charactermovement))
  (bind _returnvalue_7 (select _onrightside _returnvalue_5 _returnvalue_4))
  (Utilities|FlowControl|Sequence
    (:then_0
      (if (or (Variables|WallRunning|GetrightSide) (Variables|WallRunning|GetleftSide))
        (Variables|WallRunning|SetisJumpingOffWall true)
        (CallFunction|OffWall)
        (Utilities|FlowControl|DoOnce false :!label _label
          (:Completed
            (Character|LaunchCharacter (Math|Vector|MakeVector (.x _returnvalue_7) (.y _returnvalue_7) _jumpzvelocity) false true)
            (Variables|WallRunning|SetisJumpingOffWall false)
            (goto _label Reset)))
        (else
          (Character|Jump)
          (if (and (AI|Components|NavMovement|IsFalling (Variables|Character|GetCharacterMovement)) (Variables|Default|GetcanDoubleJump?))
            (Variables|Default|SetcanDoubleJump? false)
            (Character|LaunchCharacter (Math|Vector|MakeVector 0.0 0.0 _jumpzvelocity) false true)))))
    (:then_1
      (if (Variables|WallJump|GetstuckToWall?)
        (Variables|WallRunning|SetisJumpingOffWall true)
        (CallFunction|OffWall)
        (Utilities|FlowControl|DoOnce false :!label _label_2
          (:Completed
            (Character|LaunchCharacter (Math|Vector|MakeVector (.x _returnvalue_6) (.y _returnvalue_6) (Variables|/Script/Engine.CharacterMovementComponent|GetJumpZVelocity (Variables|Character|GetCharacterMovement))) false false)
            (Transformation|SetActorRotation (Math|Rotator|MakeRotator (.roll _returnvalue) (.pitch _returnvalue) (+ (.yaw _returnvalue) 1.8e+02)))
            (Variables|WallRunning|SetisJumpingOffWall false)
            (goto _label_2 Reset)))))))